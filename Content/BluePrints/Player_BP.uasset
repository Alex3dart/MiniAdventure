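; Player Blueprint that lets the player use items in front of them with the UseMouse input action.
; On press, it line traces the Visibility channel along the control rotation and calls OnUse on any ItemBase_BP actor hit.
; GetLocationMacro supplies both trace endpoints, offsetting the actor location by a given distance through a math expression.
; Each press also draws a temporary red debug line along the trace.
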(event `InputAction|UseMouse`
  (params (Key :type "Key Structure"))
  (bind _returnvalue (`self.GetLocationMacro` 4.0))
  (bind _returnvalue_2 (`self.GetLocationMacro` 500.0))
  (:`Pressed`
    (`KismetSystemLibrary.DrawDebugLine` _returnvalue _returnvalue_2 (struct :`R` 1.0 :`A` 1.0) 5.0 4.0)
    (bind (_outhit _returnvalue_3) (`KismetSystemLibrary.LineTraceSingle` _returnvalue _returnvalue_2 "TraceTypeQuery1"))
    (if _returnvalue_3
      (bind _asitem_base_bp (cast `/Game/BluePrints/ItemBase_BP` (`.HitActor` (`GameplayStatics.BreakHitResult` _outhit))))
      (`/Game/BluePrints/ItemBase_BP.OnUse` _asitem_base_bp))))

(fn `UserConstructionScript`)