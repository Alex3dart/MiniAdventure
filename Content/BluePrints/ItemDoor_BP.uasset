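; ItemDoor_BP is a usable door that swings open or closed each time it is used.
; OnUse flips IsOpen and calls ChangeDoorStatus, which plays the Door_TL timeline from the start to open or reverses it from the end to close.
; The timeline's RotZ track drives the relative yaw of the Scene component.
; The construction script only calls its parent; a node sizing Collision to the StaticMesh bounds is left unconnected.
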(event `ChangeDoorStatus`
  (if (`self.bIsOpen`)
    (bind (_direction _rotz) (`Timeline|Door_TL` :!via `PlayFromStart` :!label _label)
      (:`Update`
        (`SceneComponent.K2_SetRelativeRotation` (`self.Scene`) (`KismetMathLibrary.MakeRotator` 0.0 0.0 _rotz) false false)))
    (else
      (goto _label :!via `ReverseFromEnd`))))

(fn `OnUse`
  (set `self.bIsOpen` (not (`self.bIsOpen`)))
  (`self.ChangeDoorStatus`))

(fn `UserConstructionScript`
  (`parent.UserConstructionScript`))