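; Cube_BP is a cube actor whose static mesh cycles between red, green and blue materials each time it is used.
; OnUse calls the DisplayColor event, which switches on the Colores index.
; Each case prints a Spanish message naming the current color and the next one, waits a second, then applies the next material instance and advances the index, wrapping back to red.
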(event `DisplayColor`
  (switch `int` (`self.Colores`)
    (:`0`
      (`KismetSystemLibrary.PrintString` "Mi color es Rojo, se cambiara al verde en 1 seg")
      (`KismetSystemLibrary.Delay` 1.0)
      (`PrimitiveComponent.SetMaterial` (`self.StaticMesh`) 0 "/Game/Material/Color_MAT_Inst1.Color_MAT_Inst1")
      (set `self.Colores` 1))
    (:`1`
      (`KismetSystemLibrary.PrintString` "Mi color es verde,se cambiara al azul en 1 seg")
      (`KismetSystemLibrary.Delay` 1.0)
      (`PrimitiveComponent.SetMaterial` (`self.StaticMesh`) 0 "/Game/Material/Color_MAT_Inst2.Color_MAT_Inst2")
      (set `self.Colores` 2))
    (:`2`
      (`KismetSystemLibrary.PrintString` "Mi color es azul,se cambiara al rojo en 1 seg")
      (`KismetSystemLibrary.Delay` 1.0)
      (`PrimitiveComponent.SetMaterial` (`self.StaticMesh`) 0 "/Game/Material/Color_MAT_Inst.Color_MAT_Inst")
      (set `self.Colores` 0))))

(fn `OnUse`
  (`self.DisplayColor`))

(fn `UserConstructionScript`)